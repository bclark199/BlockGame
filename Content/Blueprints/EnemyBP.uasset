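; Enemy character that fires bullets on a repeating timer and can be defeated by attacks.
; A looping timer started at BeginPlay spawns EnemyBullet actors at the Arrow1 transform.
; Overlaps with actors tagged "Attack" launch it upward and reduce HP.
; When HP runs out, it changes the cube material, deactivates movement and clears the fire timer rather than being destroyed.
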(event `Fire`
  ;[1 1 1] Fire
  (`|SpawnActorFromClass` "/Game/Blueprints/Attacks/EnemyBullet.EnemyBullet_C" (`SceneComponent.K2_GetComponentToWorld` (`self.Arrow1`)) "Undefined" "OverrideRootScale"))

(event `self.ReceiveBeginPlay`
  ;[1 1 1] Repeat Fire
  (bind _returnvalue (`KismetSystemLibrary.K2_SetTimer` null "Fire" 2.0 true))
  (set `self.HP` 3))

(event `self.ReceiveActorBeginOverlap`
  (params (OtherActor :type "Actor Object Reference"))
  ;[1 1 1] Get HIt Take Damage Turn Material
  (if (`self.ActorHasTag` OtherActor "Attack")
    (`self.LaunchCharacter` (0.0 0.0 1000.0))
    ;;[1 1 1] Take damage
    (bind _output_get (set `self.HP` (- (`self.HP`) 1)))
    (if (<= _output_get 0)
      ;;[1 1 1] Die
      (`PrimitiveComponent.SetMaterial` (`self.Cube`) 0 "/Game/Geometry/Meshes/CubeMaterial.CubeMaterial")
      (`ActorComponent.SetActive` (`self.CharacterMovement`) false false)
      (`KismetSystemLibrary.K2_ClearTimerHandle` (stale `self.ReceiveBeginPlay` _returnvalue)))))

(event `self.ReceiveTick`
  (params (DeltaSeconds :type "Float (single-precision)"))
  ;[1 1 1] Get HIt Take Damage Turn Material
)

(fn `UserConstructionScript`)