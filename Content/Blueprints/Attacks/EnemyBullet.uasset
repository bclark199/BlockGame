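; Enemy homing projectile that launches upward, seeks the player character and explodes on impact.
; BeginPlay applies an upward impulse to the physics Sphere and caches the player, then Tick pulls the Sphere toward them with a constant mass-independent force.
; Hit stops homing and physics, spawns an enlarged explosion effect and destroys the fire and Sphere components, with no damage call or actor destruction.
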(event `self.ReceiveBeginPlay`
  ;[1 1 1] Launch Ball Up
  (`PrimitiveComponent.AddImpulse` (`self.Sphere`) (0.0 0.0 125000.0) "None" false)
  ;[1 1 1] Set Hero
  (set `self.Hero` (`GameplayStatics.GetPlayerCharacter` 0))
  (set `self.HeatSeak` true))

(event `self.ReceiveTick`
  (params (DeltaSeconds :type "Float (single-precision)"))
  (bind _sphere (`self.Sphere`))
  ;[1 1 1] HeatSeek
  (if (`self.heatSeak`)
    (`PrimitiveComponent.AddForce` _sphere (* (`KismetMathLibrary.GetDirectionVector` (`SceneComponent.K2_GetComponentLocation` _sphere) (`self.K2_GetActorLocation` (`self.Hero`))) (1000.0 1000.0 1000.0)) "None" true)))

(event `self.ReceiveHit`
  (params (MyComp :type "PrimitiveComponent Object Reference") (Other :type "Actor Object Reference") (OtherComp :type "PrimitiveComponent Object Reference") (bSelfMoved :type Boolean) (HitLocation :type "Vector Structure") (HitNormal :type "Vector Structure") (NormalImpulse :type "Vector Structure") (Hit :type "HitResult Structure (by ref)"))
  (bind _sphere (`self.Sphere`))
  (bind _returnvalue_location (`KismetMathLibrary.BreakTransform` (`SceneComponent.K2_GetComponentToWorld` _sphere)))
  ;[1 1 1] stop and Explode
  (set `self.HeatSeak` false)
  (`PrimitiveComponent.SetSimulatePhysics` _sphere false)
  (`|SpawnActorFromClass` "/Game/StarterContent/Blueprints/Blueprint_Effect_Explosion.Blueprint_Effect_Explosion_C" (`KismetMathLibrary.MakeTransform` _returnvalue_location (struct) (5.0 5.0 5.0)) "Undefined" "OverrideRootScale")
  (`ActorComponent.K2_DestroyComponent` (`self.P_Fire`))
  (`ActorComponent.K2_DestroyComponent` (`self.Sphere`)))

(fn `UserConstructionScript`)